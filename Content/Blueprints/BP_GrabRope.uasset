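; Rope actor built around a Cable component, currently holding only debug logic for watching the cable's length; no grab behavior is implemented here.
; On BeginPlay it caches the Cable's CableLength property as RopeLength.
; Every Tick it compares the current CableLength against that cached value and prints a different debug string for longer, equal or shorter.
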(event EventBeginPlay
  (|CallParentFunction)
  (CallFunction|InitLength))

(event Collision|EventActorBeginOverlap
  (params (OtherActor :type Actor%20Object%20Reference))
  (|CallParentFunction OtherActor) ; This node is disabled and will not be called.\nDrag off pins to build functionality.
)

(event EventTick
  (params (DeltaSeconds :type Float%20%28single-precision%29))
  (|CallParentFunction DeltaSeconds)
  (if true
    (Math|Float|CompareFloat (Variables|/Script/CableComponent.CableComponent|GetCableLength (Variables|Default|GetCable)) (Variables|Default|GetRope_Length)
      (:>
        (Development|PrintString "True"))
      (:==
        (Development|PrintString "Middle"))
      (:<
        (Development|PrintString "False")))))

(fn ConstructionScript
  (|CallParentFunction))

(fn InitLength
  (Variables|Default|SetRope_Length (Variables|/Script/CableComponent.CableComponent|GetCableLength (Variables|Default|GetCable))))