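; Pickup actor that a motion controller can grab and drop, exposing its PickupObject and a stubbed hand animation getter.
; Pickup disables physics on Base, attaches it to the given component, optionally snapping to a socket, and plays a sound at world origin.
; If already grabbed, it first forwards the pickup to PickupObject and prints its name.
; Drop re-enables physics, detaches the actor and clears the grabbed state.
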(event EventBeginPlay)

(event Collision|EventActorBeginOverlap
  (params (OtherActor :type Actor%20Object%20Reference)))

(event EventTick
  (params (DeltaSeconds :type Float%20%28single-precision%29)))

(event EventPickup
  (params (AttachTo :type Scene%20Component%20Object%20Reference))
  (bind _bsnaptosocket_ (Variables|Default|GetbSnapToSocket?))
  (bind _pickupobject (Variables|Default|GetPickupObject))
  (bind _returnvalue (select _bsnaptosocket_ "SnapToTarget" "KeepWorld"))
  (if (not (Variables|Default|GetbGrabbed?))
    _
    (else
      (Default|CallPickup _pickupobject AttachTo)
      (Development|PrintString (Utilities|GetObjectName _pickupobject))))
  (Physics|SetSimulatePhysics (Variables|Pickup|GetBase) false)
  (Transformation|AttachComponentToComponent (Variables|Pickup|GetBase) AttachTo (select (Variables|Default|GetbSnapToSocket?) (Variables|Default|GetSnapSocket) "None") _returnvalue _returnvalue "KeepWorld" false)
  (Variables|Default|SetbGrabbed? true)
  (Audio|PlaySoundatLocation (Variables|Default|Getsfx) "0, 0, 0" "0, 0, 0" 1.0 1.0 0.0 0 0 0))

(event EventDrop
  (Physics|SetSimulatePhysics (Variables|Pickup|GetBase) true)
  (Transformation|DetachFromActor "KeepWorld" "KeepWorld" "KeepWorld")
  (Variables|Default|SetbGrabbed? false))

(fn ConstructionScript)

(fn GetAnimSequence
  (params (Hand :type EControllerHand%20Enum :default "Left"))
  (return 0))

(fn GetPickupComponent
  (return (Variables|Default|GetPickupObject)))