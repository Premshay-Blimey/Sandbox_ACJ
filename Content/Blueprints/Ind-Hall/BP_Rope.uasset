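; BP_Rope is a rope actor with leftover logic for ringing a bell when pulled.
; CableCurrentLength measures the 2D distance between Base and PhysicsConstraint, which the pull logic compares against a stored length and PullLength to set IsPulling and play Bell_Single.
; That pull logic is disconnected and never runs, so live events only call the parent.
; GetPickupComponent and GetAnimSequence are empty stubs.
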(event EventBeginPlay
  (|CallParentFunction))

(event Collision|EventActorBeginOverlap
  (params (OtherActor :type Actor%20Object%20Reference))
  (|CallParentFunction OtherActor) ; This node is disabled and will not be called.\nDrag off pins to build functionality.
)

(event EventTick
  (params (DeltaSeconds :type Float%20%28single-precision%29))
  (|CallParentFunction DeltaSeconds))

(fn ConstructionScript
  (|CallParentFunction))

(fn GetPickupComponent
  (return 0))

(fn GetAnimSequence
  (params (Hand :type EControllerHand%20Enum :default "Left"))
  (return 0))

(fn CableCurrentLength
  (return (Math|Vector|Distance2D(Vector) (Transformation|GetWorldLocation (Variables|Default|GetBase)) (Transformation|GetWorldLocation (Variables|Default|GetPhysicsConstraint)))))